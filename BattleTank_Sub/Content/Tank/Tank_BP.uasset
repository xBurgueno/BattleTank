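; Player-controlled tank Blueprint that maps input to track driving, camera aiming and firing.
; On BeginPlay it registers its Barrel and Turret components through reference setters.
; Aim axes rotate the azimuth gimbal in yaw and the spring arm in pitch, scaled by delta time for frame-rate independence.
; Throttle axes drive the left and right tracks separately, and the Shoot action calls Fire.
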(event `self.ReceiveBeginPlay`
  (`self.SetBarrelReference` (`self.Barrel`))
  (`self.SetTurretReference` (`self.Turret`)))

(event `InputAxis|AImAzimuth`
  (params (AxisValue :type "Float (single-precision)"))
  ;[1 1 1] Aim Input Binding
  (`SceneComponent.K2_AddLocalRotation` (`self.AzimuthGimbal`) (`KismetMathLibrary.MakeRotator` 0.0 0.0 (* AxisValue (`GameplayStatics.GetWorldDeltaSeconds`) 100.0)) false false))

(event `InputAxis|LeftTrackThrottle`
  (params (AxisValue :type "Float (single-precision)"))
  (`TankTracks.SetThrottle` (`self.LeftTrack`) AxisValue))

(event `InputAxis|RightTrackThrottle`
  (params (AxisValue :type "Float (single-precision)"))
  (`TankTracks.SetThrottle` (`self.RightTrack`) AxisValue))

(event `InputAxis|AimElevation`
  (params (AxisValue :type "Float (single-precision)"))
  ;[1 1 1] Aim Input Binding
  (`SceneComponent.K2_AddLocalRotation` (`self.SpringArm`) (`KismetMathLibrary.MakeRotator` 0.0 (* AxisValue (`GameplayStatics.GetWorldDeltaSeconds`) 100.0)) false false))

(event `InputAction|Shoot`
  (params (Key :type "Key Structure"))
  ;[1 1 1] Aim Input Binding
  (:`Pressed`
    (`self.Fire`)))

(fn `UserConstructionScript`)